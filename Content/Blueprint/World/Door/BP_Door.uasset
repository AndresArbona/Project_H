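; BP_Door is an interactable hinged door with closed, partially open and open states that swings away from or toward zero yaw.
; OpenDoor picks the swing side from the dot product of the player's forward vector and DoorOpenLocation's forward.
; HandleDoorStates maps the current state to a slight, full or zero angle, which HandleDoorRotation approaches with FInterpTo.
; Interact starts a timer with no visible event binding, and nothing shown changes the state.
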(event `self.ReceiveBeginPlay`
  (bind _asbp_player_character (cast `/Game/Blueprint/Framework/Player/BP_PlayerCharacter` (`GameplayStatics.GetPlayerCharacter` 0)))
  (set `self.PlayerCharacterRef` _asbp_player_character))

(event `/Game/Blueprint/Framework/Interface/BI_InteractionInterface.Interact`
  (`KismetSystemLibrary.K2_SetTimerDelegate` :`Time` (`self.OpenDoorTime`)))

(event `HandleRotation`
  (params (`Set rotation` :type "Float (double-precision)"))
  ;[0.11 0.4583 0.0932] Handle Rotation
  (`self.HandleDoorRotation` `Set rotation`))

(event `HandleDoor`
  ;[0.11 0.4583 0.0932] Handle Door
  (`self.HandleDoorStates`))

(event `OpenDoor`
  (params (Player :type "/Game/Blueprint/Framework/Player/BP_PlayerCharacter Object Reference"))
  (bind _returnvalue (`self.GetPlayerRelativeLocationToTheDoor` Player))
  (if _returnvalue
    (set `self.DoorOpenSide` 1.0)
    (else
      (set `self.DoorOpenSide` -1.0))))

(fn `GetPlayerRelativeLocationToTheDoor`
  (params (self2 :type "Actor Object Reference"))
  (returns (ReturnValue :type Boolean))
  (return (> (`KismetMathLibrary.Dot_VectorVector` (`self.GetActorForwardVector` self2) (`SceneComponent.GetForwardVector` (`self.DoorOpenLocation`))) 0.0)))

(fn `HandleDoorRotation`
  (params (Target :type "Float (double-precision)"))
  (`SceneComponent.K2_SetRelativeRotation` (`self.DoorMesh`) (`KismetMathLibrary.MakeRotator` 0.0 0.0 (`KismetMathLibrary.FInterpTo` (.yaw (`SceneComponent.RelativeRotation` (`self.DoorMesh`))) Target (`GameplayStatics.GetWorldDeltaSeconds`) (`self.Interp Speed`))) false false))

(fn `HandleDoorStates`
  (switch `/Game/Blueprint/World/Door/E_DoorStates` (`self.E_DoorStates`)
    (:`NewEnumerator0`
      (`self.HandleRotation` (* 15.0 (`self.DoorOpenSide`))))
    (:`NewEnumerator1`
      (`self.HandleRotation` (* (`self.DoorOpenAngle`) (`self.DoorOpenSide`))))
    (:`NewEnumerator2`
      (`self.HandleRotation` 0.0))))

(fn `UserConstructionScript`)