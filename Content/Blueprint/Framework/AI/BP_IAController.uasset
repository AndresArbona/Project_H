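; AI controller for enemy characters that runs the enemy behavior tree and feeds perception results into its Blackboard.
; Each perception update passes through sight, hearing and prediction handlers, filtered by sense class.
; Sight sets or clears the player as TargetActor, requesting a short movement prediction on loss.
; Hearing writes TargetLocation, while the prediction result writes LastKnownLocation.
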(event `self.ReceiveBeginPlay`
  (`self.RunBehaviorTree` "/Game/Blueprint/Framework/AI/BT_EnemyCharacter.BT_EnemyCharacter"))

(event `self.AIPerception.OnTargetPerceptionUpdated`
  (params (Actor :type "Actor Object Reference") (Stimulus :type "AIStimulus Structure"))
  (`self.HandleSightSense` Actor Stimulus)
  (`self.HandleSoundSense` Actor Stimulus)
  (`self.HandlePrediction` null Stimulus))

(fn `HandlePrediction`
  (params (Actor :type "Actor Object Reference") (Stimulus :type "AIStimulus Structure"))
  (bind _returnvalue (`AIPerceptionSystem.GetSenseClassForStimulus` Stimulus))
  (if (== _returnvalue "/Script/AIModule.AISense_Prediction")
    (`BlackboardComponent.SetValueAsVector` (`self.Blackboard`) "LastKnownLocation" (`.StimulusLocation` (break `AIStimulus` (`local.Stimulus`))))))

(fn `HandleSightSense`
  (params (Actor :type "Actor Object Reference") (Stimulus :type "AIStimulus Structure"))
  (bind (_stimulus_age _stimulus_expirationage _stimulus_strength _stimulus_stimuluslocation _stimulus_receiverlocation _stimulus_tag _stimulus_bsuccessfullysensed) (break `AIStimulus` (`local.Stimulus`)))
  (bind _returnvalue (`AIPerceptionSystem.GetSenseClassForStimulus` Stimulus))
  (if (== _returnvalue "/Script/AIModule.AISense_Sight")
    (if (== (`local.Actor`) (`GameplayStatics.GetPlayerCharacter` 0))
      (`BlackboardComponent.SetValueAsObject` (`self.Blackboard`) "TargetActor" (`KismetMathLibrary.SelectObject` (`GameplayStatics.GetPlayerCharacter` 0) null _stimulus_bsuccessfullysensed))
      (if (not _stimulus_bsuccessfullysensed)
        (`AISense_Prediction.RequestPawnPredictionEvent` (`self.K2_GetPawn`) (`GameplayStatics.GetPlayerCharacter` 0) 2.0))
      (else
        (return)))
    (else
      (return))))

(fn `HandleSoundSense`
  (params (Actor :type "Actor Object Reference") (Stimulus :type "AIStimulus Structure"))
  (bind _returnvalue (`AIPerceptionSystem.GetSenseClassForStimulus` Stimulus))
  (if (== _returnvalue "/Script/AIModule.AISense_Hearing")
    (`BlackboardComponent.SetValueAsVector` (`self.Blackboard`) "TargetLocation" (`.StimulusLocation` (break `AIStimulus` (`local.Stimulus`))))))

(fn `UserConstructionScript`)