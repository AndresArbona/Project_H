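; BP_EnemyCharacter is an enemy character Blueprint that provides a melee attack through its AttackPlayer event.
; The event plays a montage on the mesh, using an IsAttacking flag to block repeat attacks until the montage completes.
; As the montage starts, a short sphere trace runs forward from AttackTrace against Pawns, with debug drawing, and applies fixed damage to the hit actor.
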(event `Attack Player`
  (bind _attacktrace (`self.AttackTrace`))
  (bind _returnvalue (`SceneComponent.K2_GetComponentLocation` _attacktrace))
  (if (not (`self.bIsAttacking`))
    (set `self.bIsAttacking` true)
    (`|PlayMontage` (`self.Mesh`)
      (:`then`
        (bind (_outhit _returnvalue_2) (`KismetSystemLibrary.SphereTraceSingleForObjects` :`Start` _returnvalue :`End` (+ _returnvalue (* (`KismetMathLibrary.GetForwardVector` (`SceneComponent.K2_GetComponentRotation` _attacktrace)) 200.0)) :`Radius` 25.0 :`ObjectTypes` (`|MakeArray` "ObjectTypeQuery3" :!type "EObjectTypeQuery Enum") :`DrawDebugType` "ForDuration"))
        (if _returnvalue_2
          (`GameplayStatics.ApplyDamage` (`.HitActor` (`GameplayStatics.BreakHitResult` _outhit)) 10.0)))
      (:`OnCompleted`
        (set `self.bIsAttacking` false)))))

(fn `UserConstructionScript`)