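; Stamina component that governs sprinting for the player character by switching its max walk speed between run and walk values.
; Each Tick, while IsRunning is set, it drains stamina by one unit per second and resets the regeneration cooldown, falling back to walk speed once empty.
; Otherwise it walks, counts down the cooldown, then refills stamina at RegenerationRate up to the maximum.
; It always targets player character 0's movement component rather than its owner's.
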(event `self.ReceiveTick`
  (params (DeltaSeconds :type "Float (single-precision)"))
  (bind _charactermovement (`Character.CharacterMovement` (`GameplayStatics.GetPlayerCharacter` 0)))
  ;[1 1 1] Logica del uso de la estamina
  (if (`self.bIsRunning`)
    (bind _bhasstamina (`self.HasStamina`))
    (`self.UseStamina` DeltaSeconds _charactermovement _bhasstamina)
    (else
      (`self.RegenerateStamina` DeltaSeconds _charactermovement))))

(fn `HasStamina`
  (returns (bHasStamina :type Boolean))
  ;[1 1 1] Revisa si usa o no estamina
  (return (> (`self.CurrentStamina`) 0.0)))

(fn `RegenerateStamina`
  (params (DeltaSeconds :type "Float (double-precision)") (CharacterMovementRef :type "CharacterMovementComponent Object Reference"))
  ;[1 1 1] Regeneracion de la estamina
  (set `CharacterMovementComponent.MaxWalkSpeed` (`self.WalkSpeed`) CharacterMovementRef)
  (bind _output_get (set `self.RegenerationCooldown` (`KismetMathLibrary.FClamp` (- (`self.RegenerationCooldown`) DeltaSeconds) 0.0 (`self.Cooldown`))))
  (if (<= _output_get 0.0)
    (set `self.CurrentStamina` (`KismetMathLibrary.FClamp` (+ (`self.CurrentStamina`) (* (`self.RegenerationRate`) DeltaSeconds)) 0.0 (`self.MaxStamina`)))))

(fn `UseStamina`
  (params (DeltaSeconds :type "Float (double-precision)") (CharacterMovementrRef :type "CharacterMovementComponent Object Reference") (bHasStamina :type Boolean))
  ;[1 1 1] Reduce la cantidad de estamina por segundos
  (if bHasStamina
    (set `self.RegenerationCooldown` (`self.Cooldown`))
    (set `self.CurrentStamina` (`KismetMathLibrary.FClamp` (- (`self.CurrentStamina`) DeltaSeconds) 0.0 (`self.MaxStamina`)))
    (set `CharacterMovementComponent.MaxWalkSpeed` (`self.RunSpeed`) CharacterMovementrRef)
    (else
      (set `CharacterMovementComponent.MaxWalkSpeed` (`self.WalkSpeed`) CharacterMovementrRef))))